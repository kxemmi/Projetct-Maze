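; Geometry Script generated-mesh actor that builds a snow mesh on top of the actors in MeshesToAddSnowTo.
; On rebuild it merges their root component meshes in world space and builds a BVH for downward raycasts from random stream-driven points within the bounds.
; Each hit adds a squashed sphere, and the result is moved into actor space.
; Optional remesh applies morphology by SnowThickness, then box-projected UVs, tangents and split normals.
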(event EventBeginPlay)

(event Collision|EventActorBeginOverlap
  (params (OtherActor :type Actor%20Object%20Reference)))

(event EventTick
  (params (DeltaSeconds :type Float%20%28single-precision%29)))

(event Events|EventOnRebuildGeneratedMesh
  (params (TargetMesh :type Dynamic%20Mesh%20Object%20Reference))
  (Variables|Default|SetTarget%20Mesh TargetMesh)
  (Utilities|FlowControl|Sequence
    (:then_0
      (bind _returnvalue (DynamicMeshActor|AllocateComputeMesh))
      (Variables|Default|SetRaycastMeshActors _returnvalue)
      (for _array_element (Variables|Default|GetMeshesToAddSnowTo)
        (bind _returnvalue_2 (DynamicMeshActor|AllocateComputeMesh))
        (bind _returnvalue_3 (GeometryScript|Scene|CopyMeshfromComponent :Component (Variables|/Script/Engine.Actor|GetRootComponent _array_element) :ToDynamicMesh _returnvalue_2 :bTransformToWorld true :Debug 0)
          (:Failure
            _)
          (:Success
            (GeometryScript|MeshEdits|AppendMesh :TargetMesh (Variables|Default|GetRaycastMeshActors) :AppendMesh _returnvalue_3 :AppendOptions "(CombineMode=EnableAllMatching)" :Debug 0)))
        (Class|DynamicMeshActor|ReleaseComputeMesh _returnvalue_2)))
    (:then_1
      (bind (_outputbvh _returnvalue_4) (Class|GeometryScriptLibraryMeshSpatial|BuildBVHforMesh (Variables|Default|GetRaycastMeshActors) 0))
      (Variables|Default|SetOutput%20BVH _outputbvh)
      (for _index (range 0 (Variables|Default|GetNumber%20of%20spheres))
        (bind _hitresult (Class|GeometryScriptLibraryMeshSpatial|FindNearestRayIntersectionwithMesh :TargetMesh (Variables|Default|GetRaycastMeshActors) :QueryBVH (Variables|Default|GetOutput%20BVH) :RayOrigin (Math|Vector|MakeVector (Math|Random|RandomFloatinRangefromStream (Variables|Default|GetStream) (.x (.min (Class|GeometryScriptLibraryMeshQueryFunctions|GetMeshBoundingBox _returnvalue_4))) (.x (.max (Class|GeometryScriptLibraryMeshQueryFunctions|GetMeshBoundingBox _returnvalue_4)))) (Math|Random|RandomFloatinRangefromStream (Variables|Default|GetStream_0) (.y (.min (Class|GeometryScriptLibraryMeshQueryFunctions|GetMeshBoundingBox _returnvalue_4))) (.y (.max (Class|GeometryScriptLibraryMeshQueryFunctions|GetMeshBoundingBox _returnvalue_4)))) (+ (- (.z (.max (Class|GeometryScriptLibraryMeshQueryFunctions|GetMeshBoundingBox _returnvalue_4))) (.z (.min (Class|GeometryScriptLibraryMeshQueryFunctions|GetMeshBoundingBox _returnvalue_4)))) 1e+01)) :RayDirection "0.000000,0.000000,-1.000000" :Debug 0)
          (:Found
            (Class|GeometryScriptLibraryMeshPrimitiveFunctions|AppendSphereBox :TargetMesh (Variables|Default|GetTarget%20Mesh) :Transform (Math|Transform|MakeTransform (.hitposition _hitresult) "0, 0, 0" "1.000000,0.500000,1.000000") :Radius 5.0 :Debug 0)))))
    (:then_2
      (GeometryScript|Transforms|TransformMesh (Variables|Default|GetTarget%20Mesh) (Math|Transform|InvertTransform (Transformation|GetActorTransform)) true 0))
    (:then_3
      (if (Variables|Default|GetRemesh)
        (bind _returnvalue_5 (Class|GeometryScriptLibraryMeshVoxelFunctions|ApplyMeshMorphology (Variables|Default|GetTarget%20Mesh) (Utilities|Struct|MakeGeometryScriptMorphologyOptions (Utilities|Struct|MakeGeometryScript3DGridParameters "GridResolution" 0.5 64) false (Utilities|Struct|MakeGeometryScript3DGridParameters "GridResolution" 0.5 64) "Dilate" (Variables|Default|GetSnow%20Thickness)) 0))
        (bind _returnvalue_6 (Class|GeometryScriptLibraryMeshUVFunctions|SetMeshUVsfromBoxProjection :TargetMesh _returnvalue_5 :BoxTransform (Math|Transform|MakeTransform "0, 0, 0" "0, 0, 0" (- (.max (Class|GeometryScriptLibraryMeshQueryFunctions|GetMeshBoundingBox _returnvalue_5)) (.min (Class|GeometryScriptLibraryMeshQueryFunctions|GetMeshBoundingBox _returnvalue_5)))) :Debug 0))
        (bind _returnvalue_7 (Class|GeometryScriptLibraryMeshNormalsFunctions|ComputeTangents :TargetMesh _returnvalue_6 :Debug 0))
        (Class|GeometryScriptLibraryMeshNormalsFunctions|ComputeSplitNormals :TargetMesh _returnvalue_7 :SplitOptions (Utilities|Struct|MakeGeometryScriptSplitNormalsOptions true 8e+01 false "(bDefaultLayer=True,ExtendedLayerIndex=0)") :Debug 0)))))

(fn ConstructionScript)